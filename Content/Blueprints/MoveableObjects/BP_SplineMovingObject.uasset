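; BP_SplineMovingObject is a moveable object that carries its Pivot along a spline, following both location and rotation.
; A timeline's Alpha maps to spline distance, with Start, Resume, Stop and Reverse controlling playback.
; The construction script applies looping, duration-based play rate and an optional override curve.
; Updates fire AtStart at zero distance and AtFinish at every other distance, as the end-of-spline check is unconnected.
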(event `Resume`
  (bind (_direction _alpha) (`Timeline|MovingObjectTimeline` :!label _label)
    (:`Update`
      (bind _returnvalue (`KismetMathLibrary.Lerp` 0.0 (`SplineComponent.GetSplineLength` (`self.Spline`)) _alpha))
      (`SceneComponent.K2_SetRelativeLocationAndRotation` (`self.Pivot`) (`SplineComponent.GetLocationAtDistanceAlongSpline` (`self.Spline`) _returnvalue "Local") (`SplineComponent.GetRotationAtDistanceAlongSpline` (`self.Spline`) _returnvalue "Local") false true)
      (if (`KismetMathLibrary.NearlyEqual_FloatFloat` _returnvalue)
        (`self.OnAtStart`)
        (elif true
          (`self.OnAtFinish`))))))

(event `Start`
  (goto _label :!via `PlayFromStart`))

(event `Stop`
  (goto _label :!via `Stop`))

(event `Reverse`
  (goto _label :!via `Reverse`))

(fn `UserConstructionScript`
  (`TimelineComponent.SetLooping` (`self.MovingObjectTimeline`) (`self.Loop`))
  (`TimelineComponent.SetPlayRate` (`self.MovingObjectTimeline`) (/ 1.0 (`self.Duration`)))
  (`/Engine/EditorBlueprintResources/StandardMacros.IsValid` (`self.OverrideCurve`)
    (:`Is Valid`
      (`TimelineComponent.SetFloatCurve` (`self.MovingObjectTimeline`) (`self.OverrideCurve`) "Alpha"))))