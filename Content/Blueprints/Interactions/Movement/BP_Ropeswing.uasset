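; Interactable rope swing that carries the side-scroller player character between two trigger points around a pivot.
; The construction script derives rope length and starting roll from pivot and trigger locations; only the current trigger has collision and enables input while active.
; Interact starts Tick, which lerps pivot roll over the summed swing angles while placing the levitating character along the rope.
; On arrival, it releases the character and swaps triggers for the return swing.
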(event `self.ReceiveBeginPlay`
  (set `self.IsActive` (`self.IsActiveFromStart`))
  (`self.SetSumOfAngles`)
  (bind _asbp_side_scroller_character (cast `/Game/Blueprints/Characters/BP_SideScrollerCharacter` (`GameplayStatics.GetPlayerCharacter` 0)))
  (set `self.Character` _asbp_side_scroller_character))

(event `self.TriggerPoint1.OnComponentBeginOverlap`
  (params (OverlappedComponent :type "PrimitiveComponent Object Reference") (OtherActor :type "Actor Object Reference") (OtherComp :type "PrimitiveComponent Object Reference") (OtherBodyIndex :type Integer) (bFromSweep :type Boolean) (SweepResult :type "HitResult Structure (by ref)"))
  (if (`self.IsActive`) :!label _label
    (`self.EnableInput` (`GameplayStatics.GetPlayerController` 0))))

(event `self.TriggerPoint2.OnComponentBeginOverlap`
  (params (OverlappedComponent :type "PrimitiveComponent Object Reference") (OtherActor :type "Actor Object Reference") (OtherComp :type "PrimitiveComponent Object Reference") (OtherBodyIndex :type Integer) (bFromSweep :type Boolean) (SweepResult :type "HitResult Structure (by ref)"))
  (goto _label))

(event `self.TriggerPoint1.OnComponentEndOverlap`
  (params (OverlappedComponent :type "PrimitiveComponent Object Reference") (OtherActor :type "Actor Object Reference") (OtherComp :type "PrimitiveComponent Object Reference") (OtherBodyIndex :type Integer))
  (if (`self.IsActive`) :!label _label_2
    (`self.DisableInput` (`GameplayStatics.GetPlayerController` 0))))

(event `self.TriggerPoint2.OnComponentEndOverlap`
  (params (OverlappedComponent :type "PrimitiveComponent Object Reference") (OtherActor :type "Actor Object Reference") (OtherComp :type "PrimitiveComponent Object Reference") (OtherBodyIndex :type Integer))
  (goto _label_2))

(event `InputAction|Interact` :consume false :overrideparent false
  (params (Key :type "Key Structure"))
  (:`Pressed`
    (bind _caninteract (`self.CanInteract`))
    (if _caninteract
      (set `self.InProgress` true)
      (`self.SetActorTickEnabled` true)
      (`/Game/Blueprints/Characters/BP_SideScrollerCharacter.Set Levitating` (`self.Character`) true))))

(event `self.ReceiveTick`
  (params (DeltaSeconds :type "Float (single-precision)"))
  (if (`self.InProgress`)
    (bind _rotation (`self.RotateRope` DeltaSeconds)
      (:`Finish`
        (`self.SetActorTickEnabled` false)
        (set `self.InProgress` false)
        (set `self.Progress` 0.0)
        (`self.SetCurrentTrigger` (select `int` (`self.CurrentActive`) :`0` 1 :`1` 0))
        (`/Game/Blueprints/Characters/BP_SideScrollerCharacter.Set Levitating` (`self.Character`) false)
        (`self.K2_SetActorRotation` (`self.Character`) (`KismetMathLibrary.MakeRotator` 0.0 0.0 (* (`self.FindDirection`) -90.0)) false))
      (:`Update`
        (`self.SetCharacterPositionAndRotation` _rotation)))))

(fn `CanInteract`
  (returns (CanInteract :type Boolean))
  (bind _caninteract (`parent.CanInteract`))
  (return (and _caninteract (`self.IsActive`) (not (`self.InProgress`)))))

(fn `FindDirection`
  (returns (ReturnValue :type "Float (double-precision)"))
  (bind (_current _opposite) (`self.GetTriggerLocations`))
  (return (`KismetMathLibrary.SignOfFloat` (- (.y _opposite) (.y _current)))))

(fn `FindRopeRotation`
  (params (Target :type "Vector Structure (by ref)"))
  (returns (Rotation :type "Rotator Structure"))
  (bind (_pivotpoint_x _pivotpoint_y) (`KismetMathLibrary.BreakVector` (`self.PivotPoint`)))
  (return (`KismetMathLibrary.MakeRotator` (* (`KismetMathLibrary.DegAcos` (`KismetMathLibrary.Dot_VectorVector` (`KismetMathLibrary.Normal` Target) (`KismetMathLibrary.Normal` (* (`KismetMathLibrary.Vector_Down`) (`self.PivotPoint`))))) (`KismetMathLibrary.SignOfFloat` (- _pivotpoint_y (.y Target)))))))

(fn `GetTriggerLocations`
  (returns (Current :type "Vector Structure") (Opposite :type "Vector Structure"))
  (return (select `int` (`self.CurrentActive`) :`0` (`self.TriggerPointLocation1`) :`1` (`self.TriggerPointLocation2`)) (select `int` (`self.CurrentActive`) :`0` (`self.TriggerPointLocation2`) :`1` (`self.TriggerPointLocation1`))))

(fn `GetTriggers`
  (returns (Current :type "BoxComponent Object Reference") (Opposite :type "BoxComponent Object Reference"))
  (return (select `int` (`self.CurrentActive`) :`0` (`self.TriggerPoint1`) :`1` (`self.TriggerPoint2`)) (select `int` (`self.CurrentActive`) :`0` (`self.TriggerPoint2`) :`1` (`self.TriggerPoint1`))))

(fn `SetCharacterPositionAndRotation`
  (params (RopeRotation :type "Rotator Structure"))
  (bind _returnvalue (`self.FindDirection`))
  (`self.K2_SetActorLocation` (`self.Character`) (+ (* (`KismetMathLibrary.Normal` (* (`SceneComponent.GetUpVector` (`self.Pivot`)) -1.0)) (- (`self.RopeLength`) (`self.GrabOffsetFromEnd`))) (`SceneComponent.K2_GetComponentLocation` (`self.Pivot`))) false false)
  (`self.K2_SetActorRotation` (`self.Character`) (`KismetMathLibrary.MakeRotator` 0.0 (* (.roll RopeRotation) _returnvalue -1.0) (* _returnvalue 90.0)) false))

(fn `SetCurrentTrigger`
  (params (Index :type Integer))
  (bind _output_get (set `self.CurrentActive` Index))
  (`PrimitiveComponent.SetCollisionEnabled` (select `int` _output_get :`0` (`self.TriggerPoint1`) :`1` (`self.TriggerPoint2`)) "QueryAndPhysics")
  (`PrimitiveComponent.SetCollisionEnabled` (select `int` _output_get :`0` (`self.TriggerPoint2`) :`1` (`self.TriggerPoint1`)) "NoCollision"))

(fn `SetSumOfAngles`
  (bind (_current _opposite) (`self.GetTriggerLocations`))
  (bind _rotation_roll (`KismetMathLibrary.BreakRotator` (`self.FindRopeRotation` (- _current (`self.PivotPoint`)))))
  (bind _rotation_roll_2 (`KismetMathLibrary.BreakRotator` (`self.FindRopeRotation` (- _opposite (`self.PivotPoint`)))))
  (set `self.SumOfAngles` (+ (`KismetMathLibrary.Abs` _rotation_roll) (`KismetMathLibrary.Abs` _rotation_roll_2))))

(fn `UserConstructionScript`
  (`self.SetCurrentTrigger` (`self.StartActiveTrigger`))
  (`SceneComponent.K2_SetRelativeLocation` (`self.TriggerPoint1`) (`self.TriggerPointLocation1`) false false)
  (`SceneComponent.K2_SetRelativeLocation` (`self.TriggerPoint2`) (`self.TriggerPointLocation2`) false false)
  (`SceneComponent.K2_SetWorldLocation` (`self.Pivot`) (+ (`self.K2_GetActorLocation`) (`self.PivotPoint`)) false false)
  (bind _output_get (set `self.RopeLength` (`KismetMathLibrary.VSize` (- (`self.GetTriggerLocations`) (`self.PivotPoint`)))))
  (`SplineMeshComponent.SetEndPosition` (`self.Rope`) (`KismetMathLibrary.MakeVector` _output_get) true)
  (`SceneComponent.K2_SetRelativeRotation` (`self.Pivot`) (`self.FindRopeRotation` (- (`self.GetTriggerLocations`) (`self.PivotPoint`))) false false))