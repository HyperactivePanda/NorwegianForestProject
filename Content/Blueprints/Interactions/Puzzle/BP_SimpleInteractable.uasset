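; BP_SimpleInteractable is a puzzle interaction actor that responds to the Interact input action near its trigger.
; While active, its trigger enables input for player controller 0 on any overlap and disables it on overlap end.
; A press calls CanInteract, then CallOnInteract if allowed, and turns off trigger collision unless it is reusable.
; StartAsActive sets the initial active state at BeginPlay.
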(event `self.ReceiveBeginPlay`
  (set `self.IsActive` (`self.StartAsActive`)))

(event `self.Trigger.OnComponentBeginOverlap`
  (params (OverlappedComponent :type "PrimitiveComponent Object Reference") (OtherActor :type "Actor Object Reference") (OtherComp :type "PrimitiveComponent Object Reference") (OtherBodyIndex :type Integer) (bFromSweep :type Boolean) (SweepResult :type "HitResult Structure (by ref)"))
  (if (`self.IsActive`)
    (`self.EnableInput` (`GameplayStatics.GetPlayerController` 0))))

(event `self.Trigger.OnComponentEndOverlap`
  (params (OverlappedComponent :type "PrimitiveComponent Object Reference") (OtherActor :type "Actor Object Reference") (OtherComp :type "PrimitiveComponent Object Reference") (OtherBodyIndex :type Integer))
  (if (`self.IsActive`)
    (`self.DisableInput` (`GameplayStatics.GetPlayerController` 0))))

(event `InputAction|Interact` :consume false :overrideparent false
  (params (Key :type "Key Structure"))
  (:`Pressed`
    (bind _caninteract (`self.CanInteract`))
    (if _caninteract
      (`self.OnInteract`)
      (if (not (`self.Reusable`))
        (`PrimitiveComponent.SetCollisionEnabled` (`self.Trigger`) "NoCollision")))))

(fn `UserConstructionScript`)