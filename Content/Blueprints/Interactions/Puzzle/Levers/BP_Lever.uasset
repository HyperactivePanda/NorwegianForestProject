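; BP_Lever is an interactable puzzle lever whose pivot pitch the player drives with the Rotate axis while pulling.
; Interact toggles pulling through a FlipFlop, unless the lever is one-way and has already been pulled once.
; SetRotation wraps the pivot's pitch to a signed angle, adds scaled input, clamps between Start and End in either order, and passes it to the parent.
; Initialize sets the Start angle, and GetLeverLimits exposes both limits.
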(event `InputAction|Interact`
  (params (Key :type "Key Structure"))
  (:`Pressed`
    (if (`KismetMathLibrary.BooleanNAND` (`self.OneWay`) (`self.PulledOnce`))
      (`/Engine/EditorBlueprintResources/StandardMacros.FlipFlop`
        (:`A`
          (`self.EnablePulling`))
        (:`B`
          (`self.DisablePulling`))))))

(event `InputAxis|Rotate`
  (params (AxisValue :type "Float (single-precision)"))
  (if (`self.Pulling`)
    (`self.SetRotation` AxisValue)))

(fn `GetLeverLimits`
  (returns (Start :type "Float (double-precision)") (End :type "Float (double-precision)"))
  (return (`self.Start`) (`self.End`)))

(fn `Initialize`
  (`parent.Initialize`)
  (`self.SetRotation` (`self.Start`)))

(fn `SetRotation`
  (params (Pitch :type "Float (double-precision)"))
  (bind _start (`self.Start`))
  (bind _end (`self.End`))
  (bind _returnvalue (< _start _end))
  (bind (_relativerotation_roll _relativerotation_pitch) (`KismetMathLibrary.BreakRotator` (`SceneComponent.RelativeRotation` (`self.Pivot`))))
  (`parent.SetRotation` (`KismetMathLibrary.FClamp` (+ (* Pitch (`self.PullingSpeed`)) (select `bool` (>= _relativerotation_pitch 270.0) :`false` _relativerotation_pitch :`true` (- _relativerotation_pitch 360.0))) (select `bool` _returnvalue :`false` _end :`true` _start) (select `bool` _returnvalue :`false` _start :`true` _end))))

(fn `UserConstructionScript`)