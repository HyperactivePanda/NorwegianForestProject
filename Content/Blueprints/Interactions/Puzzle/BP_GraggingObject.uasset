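; Draggable puzzle object that the side-scroller player character can drag along a limited track.
; A trigger enables input and dragging while overlapped, and Interact flip-flops dragging, which sets the character's drag state, mesh collision and actor tick.
; Each tick the mesh follows the player at the offset captured on grab, with relative X clamped between Start and End.
; When clamping breaks that offset, the character is snapped back to restore it.
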(event `self.Trigger.OnComponentBeginOverlap`
  (params (OverlappedComponent :type "PrimitiveComponent Object Reference") (OtherActor :type "Actor Object Reference") (OtherComp :type "PrimitiveComponent Object Reference") (OtherBodyIndex :type Integer) (bFromSweep :type Boolean) (SweepResult :type "HitResult Structure (by ref)"))
  (set `self.CanDrag` true)
  (`self.EnableInput` (`GameplayStatics.GetPlayerController` 0)))

(event `self.Trigger.OnComponentEndOverlap`
  (params (OverlappedComponent :type "PrimitiveComponent Object Reference") (OtherActor :type "Actor Object Reference") (OtherComp :type "PrimitiveComponent Object Reference") (OtherBodyIndex :type Integer))
  (set `self.CanDrag` false)
  (`self.DisableInput` (`GameplayStatics.GetPlayerController` 0)))

(event `InputAction|Interact`
  (params (Key :type "Key Structure"))
  (:`Pressed`
    (`/Engine/EditorBlueprintResources/StandardMacros.FlipFlop`
      (:`A`
        (`self.Enable Dragging`))
      (:`B`
        (`self.DisableDragging`)))))

(event `self.ReceiveTick`
  (params (DeltaSeconds :type "Float (single-precision)"))
  (`self.MovePosition`)
  (`self.ClampPosition`)
  (`self.ClampCharacterPosition`))

(fn `ClampCharacterPosition`
  (if (!= (`self.GetDelta`) (`self.Delta`))
    (`self.K2_SetActorLocation` (`GameplayStatics.GetPlayerCharacter` 0) (- (`SceneComponent.K2_GetComponentLocation` (`self.StaticMesh`)) (`self.Delta`)) false false)))

(fn `ClampPosition`
  (bind _start_x (`KismetMathLibrary.BreakVector` (`self.Start`)))
  (bind _end_x (`KismetMathLibrary.BreakVector` (`self.End`)))
  (bind (_relativelocation_x _relativelocation_y _relativelocation_z) (`KismetMathLibrary.BreakVector` (`SceneComponent.RelativeLocation` (`self.StaticMesh`))))
  (`SceneComponent.K2_SetRelativeLocation` (`self.StaticMesh`) (`KismetMathLibrary.MakeVector` (`KismetMathLibrary.FClamp` _relativelocation_x _start_x _end_x) _relativelocation_y _relativelocation_z) false false))

(fn `DisableDragging`
  (if (`self.CanDrag`)
    (bind _asbp_side_scroller_character (cast `/Game/Blueprints/Characters/BP_SideScrollerCharacter` (`GameplayStatics.GetPlayerCharacter` 0)))
    (`/Game/Blueprints/Characters/BP_SideScrollerCharacter.SetDragging` _asbp_side_scroller_character false)
    (set `self.Delta` (0.0 0.0 0.0))
    (`PrimitiveComponent.SetCollisionEnabled` (`self.StaticMesh`) "QueryAndPhysics")
    (`self.SetActorTickEnabled` false)))

(fn `Enable Dragging`
  (if (`self.CanDrag`)
    (bind _asbp_side_scroller_character (cast `/Game/Blueprints/Characters/BP_SideScrollerCharacter` (`GameplayStatics.GetPlayerCharacter` 0)))
    (`/Game/Blueprints/Characters/BP_SideScrollerCharacter.SetDragging` _asbp_side_scroller_character true)
    (set `self.Delta` (`self.GetDelta`))
    (`PrimitiveComponent.SetCollisionEnabled` (`self.StaticMesh`) "NoCollision")
    (`self.SetActorTickEnabled` true)))

(fn `GetDelta`
  (returns (Delta :type "Vector Structure"))
  (return (- (`SceneComponent.K2_GetComponentLocation` (`self.StaticMesh`)) (`self.K2_GetActorLocation` (`GameplayStatics.GetPlayerCharacter` 0)))))

(fn `MovePosition`
  (`SceneComponent.K2_SetWorldLocation` (`self.StaticMesh`) (+ (`self.K2_GetActorLocation` (`GameplayStatics.GetPlayerCharacter` 0)) (`self.Delta`)) false false))

(fn `UserConstructionScript`)