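; Player controller that handles pausing, checkpoint spawning and the game-over flow.
; On begin play it unpauses and moves the controlled pawn to the current checkpoint's saved location and rotation from BP_GameInstance.
; The menu input pauses the game, shows the cursor and opens WB_PauseMenu.
; HandleOnDead shows WB_GameOver, after which any key press removes it and calls LoadGame on the game instance.
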(event `self.ReceiveBeginPlay`
  (`self.Resume`)
  (`self.SpawnAtCheckPoint`))

(event `InputAction|OpenMenu`
  (params (Key :type "Key Structure"))
  (:`Pressed`
    (set `self.bShowMouseCursor` true)
    (`GameplayStatics.SetGamePaused` true)
    (bind _returnvalue (`|CreateWidget` "/Game/UI/PauseMenu/WB_PauseMenu.WB_PauseMenu_C"))
    (`UserWidget.AddToViewport` _returnvalue 0)))

(event `Resume`
  (set `self.bShowMouseCursor` false)
  (`GameplayStatics.SetGamePaused` false))

(event `SpawnAtCheckPoint`
  (bind _asbp_game_instance (cast `/Game/Blueprints/GameInstance/BP_GameInstance` (`GameplayStatics.GetGameInstance`)))
  (bind (_checkpoint _success) (`/Game/Blueprints/GameInstance/BP_GameInstance.GetCurrentCheckPoint` _asbp_game_instance))
  (if _success
    (bind (_worldname _characterlocation _characterrotation) (break `/Game/Blueprints/SaveGame/CheckPoint/ST_CheckPointData` _checkpoint))
    (`self.K2_SetActorLocationAndRotation` (`self.K2_GetPawn`) _characterlocation _characterrotation false false)))

(event `HandleOnDead`
  (bind _returnvalue (`|CreateWidget` "/Game/UI/GameOver/WB_GameOver.WB_GameOver_C"))
  (bind _output_get (set `self.GameOverWidget` _returnvalue))
  (`UserWidget.AddToViewport` _output_get 0))

(event `Key|AnyKey` :consume false :overrideparent false
  (params (Key :type "Key Structure"))
  (:`Pressed`
    (`/Engine/EditorBlueprintResources/StandardMacros.IsValid` (`self.GameOverWidget`)
      (:`Is Valid`
        (`Widget.RemoveFromParent` (`self.GameOverWidget`))
        (set `self.GameOverWidget` null)
        (bind _asbp_game_instance (cast `/Game/Blueprints/GameInstance/BP_GameInstance` (`GameplayStatics.GetGameInstance`)))
        (`/Game/Blueprints/GameInstance/BP_GameInstance.LoadGame` _asbp_game_instance)))))

(fn `UserConstructionScript`)