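; BP_CheckPoint is a checkpoint actor that saves the game when the side-scroller character overlaps its Trigger.
; It packs WorldName and the SpawnPoint component's location and rotation into checkpoint data and passes it to BP_GameInstance's SaveGame.
; A DoOnce precedes the character cast, so the first overlap by any actor consumes it.
; The OneTime-based reset is unconnected and never runs.
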(event `self.Trigger.OnComponentBeginOverlap`
  (params (OverlappedComponent :type "PrimitiveComponent Object Reference") (OtherActor :type "Actor Object Reference") (OtherComp :type "PrimitiveComponent Object Reference") (OtherBodyIndex :type Integer) (bFromSweep :type Boolean) (SweepResult :type "HitResult Structure (by ref)"))
  (`/Engine/EditorBlueprintResources/StandardMacros.DoOnce` false
    (:`Completed`
      (cast `/Game/Blueprints/Characters/BP_SideScrollerCharacter` OtherActor)
      (bind _asbp_game_instance (cast `/Game/Blueprints/GameInstance/BP_GameInstance` (`GameplayStatics.GetGameInstance`)))
      (bind _st_checkpointdata (`self.CreateCheckPointData`))
      (`/Game/Blueprints/GameInstance/BP_GameInstance.SaveGame` _asbp_game_instance _st_checkpointdata))))

(fn `CreateCheckPointData`
  (returns (ST_CheckPointData :type "/Game/Blueprints/SaveGame/CheckPoint/ST_CheckPointData Structure"))
  (bind _spawnpoint (`self.SpawnPoint`))
  (return (make `/Game/Blueprints/SaveGame/CheckPoint/ST_CheckPointData` (`self.WorldName`) (`SceneComponent.K2_GetComponentLocation` _spawnpoint) (`SceneComponent.K2_GetComponentRotation` _spawnpoint))))

(fn `UserConstructionScript`)