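; Base puzzle lever for the side-scroller, which the player can pull while overlapping its trigger.
; The trigger toggles input and CanPull, which gates functions that set the character's pulling state and switch mesh collision.
; SetRotation pitches the pivot, reports normalized pull progress, and signals when either limit is reached.
; Initialize, run at construction, and GetLeverLimits are stubs, apparently for child levers to override.
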(event `self.Trigger.OnComponentBeginOverlap`
  (params (OverlappedComponent :type "PrimitiveComponent Object Reference") (OtherActor :type "Actor Object Reference") (OtherComp :type "PrimitiveComponent Object Reference") (OtherBodyIndex :type Integer) (bFromSweep :type Boolean) (SweepResult :type "HitResult Structure (by ref)"))
  (set `self.CanPull` true)
  (`self.EnableInput` (`GameplayStatics.GetPlayerController` 0)))

(event `self.Trigger.OnComponentEndOverlap`
  (params (OverlappedComponent :type "PrimitiveComponent Object Reference") (OtherActor :type "Actor Object Reference") (OtherComp :type "PrimitiveComponent Object Reference") (OtherBodyIndex :type Integer))
  (set `self.CanPull` false)
  (`self.DisableInput` (`GameplayStatics.GetPlayerController` 0)))

(fn `DisablePulling`
  (if (`self.CanPull`)
    (bind _asbp_side_scroller_character (cast `/Game/Blueprints/Characters/BP_SideScrollerCharacter` (`GameplayStatics.GetPlayerCharacter` 0)))
    (`/Game/Blueprints/Characters/BP_SideScrollerCharacter.SetPulling` _asbp_side_scroller_character false)
    (`PrimitiveComponent.SetCollisionEnabled` (`self.StaticMesh`) "QueryAndPhysics")
    (set `self.Pulling` false)))

(fn `EnablePulling`
  (if (`self.CanPull`)
    (bind _asbp_side_scroller_character (cast `/Game/Blueprints/Characters/BP_SideScrollerCharacter` (`GameplayStatics.GetPlayerCharacter` 0)))
    (`/Game/Blueprints/Characters/BP_SideScrollerCharacter.SetPulling` _asbp_side_scroller_character true)
    (`PrimitiveComponent.SetCollisionEnabled` (`self.StaticMesh`) "NoCollision")
    (set `self.Pulling` true)))

(fn `GetLeverLimits`
  (returns (Start :type "Float (double-precision)") (End :type "Float (double-precision)"))
  (return 0.0 0.0))

(fn `Initialize`)

(fn `SetRotation`
  (params (Pitch :type "Float (double-precision)"))
  (bind (_relativerotation_roll _relativerotation_pitch _relativerotation_yaw) (`KismetMathLibrary.BreakRotator` (`SceneComponent.RelativeRotation` (`self.Pivot`))))
  (`SceneComponent.K2_SetRelativeRotation` (`self.Pivot`) (`KismetMathLibrary.MakeRotator` _relativerotation_roll Pitch _relativerotation_yaw) false false)
  (bind (_start _end) (`self.GetLeverLimits`))
  (bind _returnvalue (`KismetMathLibrary.Abs` _start))
  (`self.OnLeverPull` (/ (+ _returnvalue Pitch) (+ _end _returnvalue)))
  (if (`KismetMathLibrary.NearlyEqual_FloatFloat` _start Pitch)
    (`self.OnLeverStart`)
    (elif (`KismetMathLibrary.NearlyEqual_FloatFloat` _end Pitch)
      (`self.OnLeverEnd`))))

(fn `UserConstructionScript`
  (`self.Initialize`))