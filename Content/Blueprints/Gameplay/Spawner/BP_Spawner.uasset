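; BP_Spawner is a spawner that places actors of a configurable class at a set transform on a looping timer.
; SetActive pauses or resumes the timer, which is paused at BeginPlay unless IsActiveFromStart is set.
; Each tick of the timer creates and tags a new actor until the pool is full.
; It then recycles pooled actors round-robin, resetting only their transform.
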(event `self.ReceiveBeginPlay`
  (bind _returnvalue (`KismetSystemLibrary.K2_SetTimerDelegate` (delegate `OnSpawn`) (`self.SpawnRate`) true))
  (bind _output_get (set `self.TimerHandle` _returnvalue))
  (if (not (`self.IsActiveFromStart`))
    (`KismetSystemLibrary.K2_PauseTimerHandle` _output_get)))

(event `OnSpawn`
  (`self.SpawnActor`))

(event `SetActive`
  (params (IsActive :type Boolean))
  (bind _timerhandle (`self.TimerHandle`))
  (if IsActive
    (`KismetSystemLibrary.K2_UnPauseTimerHandle` _timerhandle)
    (else
      (`KismetSystemLibrary.K2_PauseTimerHandle` _timerhandle))))

(fn `CreateActor`
  (returns (Actor :type "Actor Object Reference"))
  (bind _returnvalue (`|SpawnActorFromClass` (`self.ActorClass`) (`self.SpawnTransform`) "Undefined" "OverrideRootScale" null null))
  (set `Actor.Tags` (`self.TagsToAdd`) _returnvalue)
  (return _returnvalue))

(fn `ResetActor`
  (params (Actor :type "Actor Object Reference"))
  (`self.K2_SetActorTransform` Actor (`self.SpawnTransform`) false false))

(fn `SpawnActor`
  (locals (ActorToReturn :type "Actor Object Reference"))
  (if (== (`KismetArrayLibrary.Array_Length` (`self.ActorsPool`)) (`self.ObjectPullSize`))
    (bind _output_get (set `local.ActorToReturn` (`|GetArrayItem` (`self.ActorsPool`) (`self.ActorIndexToRespawn`))))
    (`self.ResetActor` _output_get)
    (bind _result (`/Engine/EditorBlueprintResources/StandardMacros.IncrementInt` (`self.ActorIndexToRespawn`))
      (:`  `
        (set `self.ActorIndexToRespawn` (mod _result (`self.ObjectPullSize`)))))
    (else
      (bind _actor (`self.CreateActor`))
      (`KismetArrayLibrary.Array_Add` (`self.ActorsPool`) _actor))))

(fn `UserConstructionScript`)