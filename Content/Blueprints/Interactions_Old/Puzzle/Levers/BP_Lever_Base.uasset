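; Base class for puzzle levers that the side-scroller character pulls, with an optional one-way mode that locks after reaching the end.
; An overlap trigger gates activity and input, while EnablePulling and DisablePulling toggle the character's pulling state and lever mesh collision.
; SetRotation pitches the pivot and broadcasts normalized progress plus start and end events.
; Initialize and GetLeverLimits are stubs, apparently for child levers to override.
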(event `self.Trigger.OnComponentBeginOverlap`
  (params (OverlappedComponent :type "PrimitiveComponent Object Reference") (OtherActor :type "Actor Object Reference") (OtherComp :type "PrimitiveComponent Object Reference") (OtherBodyIndex :type Integer) (bFromSweep :type Boolean) (SweepResult :type "HitResult Structure (by ref)"))
  (set `self.IsActive` true)
  (`self.EnableInput` (`GameplayStatics.GetPlayerController` 0)))

(event `self.Trigger.OnComponentEndOverlap`
  (params (OverlappedComponent :type "PrimitiveComponent Object Reference") (OtherActor :type "Actor Object Reference") (OtherComp :type "PrimitiveComponent Object Reference") (OtherBodyIndex :type Integer))
  (set `self.IsActive` false)
  (`self.DisableInput` (`GameplayStatics.GetPlayerController` 0)))

(event `self.ReceiveBeginPlay`
  (add `self.OnLeverEnd` (delegate `OnLeverEnd_Event`)))

(event `OnLeverEnd_Event`
  (set `self.PulledOnce` true)
  (if (`self.OneWay`)
    (`PrimitiveComponent.SetCollisionEnabled` (`self.Trigger`) "NoCollision")))

(fn `CanInteract`
  (returns (CanInteract :type Boolean))
  (bind _caninteract (`parent.CanInteract`))
  (return (and _caninteract (`KismetMathLibrary.BooleanNAND` (`self.OneWay`) (`self.PulledOnce`)) (not (`self.InProgress`)))))

(fn `DisablePulling`
  (bind _asbp_side_scroller_character (cast `/Game/Blueprints/Characters/BP_SideScrollerCharacter` (`GameplayStatics.GetPlayerCharacter` 0)))
  (`/Game/Blueprints/Characters/BP_SideScrollerCharacter.SetPulling` _asbp_side_scroller_character false)
  (`PrimitiveComponent.SetCollisionEnabled` (`self.StaticMesh`) "QueryAndPhysics")
  (set `self.InProgress` false))

(fn `EnablePulling`
  (if (and (`self.IsActive`) (`KismetMathLibrary.BooleanNAND` (`self.OneWay`) (`self.PulledOnce`)))
    (bind _asbp_side_scroller_character (cast `/Game/Blueprints/Characters/BP_SideScrollerCharacter` (`GameplayStatics.GetPlayerCharacter` 0)))
    (`/Game/Blueprints/Characters/BP_SideScrollerCharacter.SetPulling` _asbp_side_scroller_character true)
    (`PrimitiveComponent.SetCollisionEnabled` (`self.StaticMesh`) "NoCollision")
    (set `self.InProgress` true)))

(fn `GetLeverLimits`
  (returns (Start :type "Float (double-precision)") (End :type "Float (double-precision)"))
  (return 0.0 0.0))

(fn `Initialize`)

(fn `SetRotation`
  (params (Pitch :type "Float (double-precision)"))
  (bind (_relativerotation_roll _relativerotation_pitch _relativerotation_yaw) (`KismetMathLibrary.BreakRotator` (`SceneComponent.RelativeRotation` (`self.Pivot`))))
  (`SceneComponent.K2_SetRelativeRotation` (`self.Pivot`) (`KismetMathLibrary.MakeRotator` _relativerotation_roll Pitch _relativerotation_yaw) false false)
  (bind (_start _end) (`self.GetLeverLimits`))
  (bind _returnvalue (`KismetMathLibrary.Abs` _start))
  (`self.OnLeverPull` (/ (+ _returnvalue Pitch) (+ _end _returnvalue)))
  (if (`KismetMathLibrary.NearlyEqual_FloatFloat` _start Pitch)
    (`self.OnLeverStart`)
    (elif (`KismetMathLibrary.NearlyEqual_FloatFloat` _end Pitch)
      (`self.OnLeverEnd`)
      (if (`self.OneWay`)
        (`self.DisablePulling`)))))

(fn `UserConstructionScript`
  (`self.Initialize`))