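; Animated puzzle lever that the player toggles with the Interact input, extending a parent lever Blueprint.
; Each permitted interaction enables pulling and alternately plays or reverses a timeline, setting rotation from PullingCurve at the playback position and disabling pulling when finished.
; Initialization fits the timeline length to the curve, applies the starting rotation and caches the curve's end values as the lever limits.
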(event `InputAction|Interact` :consume false :overrideparent false
  (params (Key :type "Key Structure"))
  (:`Pressed`
    (bind _caninteract (`self.CanInteract`))
    (if _caninteract
      (`self.OnInteract`)
      (`self.EnablePulling`)
      (`/Engine/EditorBlueprintResources/StandardMacros.FlipFlop`
        (:`A`
          (`Timeline|PullingTimeline` :!label _label
            (:`Update`
              (`self.SetRotation` (`CurveFloat.GetFloatValue` (`self.PullingCurve`) (`TimelineComponent.GetPlaybackPosition` (`self.PullingTimeline`)))))
            (:`Finished`
              (`self.DisablePulling`))))
        (:`B`
          (goto _label :!via `Reverse`))))))

(event `OnInteract`)

(fn `GetLeverLimits`
  (returns (Start :type "Float (double-precision)") (End :type "Float (double-precision)"))
  (return (`self.Start`) (`self.End`)))

(fn `Initialize`
  (bind _pullingcurve (`self.PullingCurve`))
  (bind (_mintime _maxtime) (`CurveBase.GetTimeRange` _pullingcurve))
  (`parent.Initialize`)
  (`TimelineComponent.SetFloatCurve` (`self.PullingTimeline`) _pullingcurve "None")
  (`TimelineComponent.SetTimelineLength` (`self.PullingTimeline`) _maxtime)
  (bind _output_get (set `self.Start` (`CurveFloat.GetFloatValue` (`self.PullingCurve`) 0.0)))
  (`self.SetRotation` _output_get)
  (set `self.End` (`CurveFloat.GetFloatValue` (`self.PullingCurve`) _maxtime)))

(fn `UserConstructionScript`)