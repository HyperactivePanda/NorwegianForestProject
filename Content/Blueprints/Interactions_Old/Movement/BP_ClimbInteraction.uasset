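; Climb interaction actor that carries the side-scroller character along a straight line from a start to an end point.
; Overlapping the trigger while active enables input, and pressing Interact sets the character levitating, facing the climb, at the start.
; Tick moves it at constant speed until a dot-product test detects passing the end.
; It then teleports to the destination, stops levitating, and the interaction stays active only if reusable.
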(event `self.ReceiveBeginPlay`
  (`self.SetActive` (`self.StartAsActive`)))

(event `self.InteractionTrigger.OnComponentBeginOverlap`
  (params (OverlappedComponent :type "PrimitiveComponent Object Reference") (OtherActor :type "Actor Object Reference") (OtherComp :type "PrimitiveComponent Object Reference") (OtherBodyIndex :type Integer) (bFromSweep :type Boolean) (SweepResult :type "HitResult Structure (by ref)"))
  (if (`self.IsActive`)
    (`self.EnableInput` (`GameplayStatics.GetPlayerController` 0))))

(event `self.InteractionTrigger.OnComponentEndOverlap`
  (params (OverlappedComponent :type "PrimitiveComponent Object Reference") (OtherActor :type "Actor Object Reference") (OtherComp :type "PrimitiveComponent Object Reference") (OtherBodyIndex :type Integer))
  (if (`self.IsActive`)
    (`self.DisableInput` (`GameplayStatics.GetPlayerController` 0))))

(event `InputAction|Interact` :consume false :overrideparent false
  (params (Key :type "Key Structure"))
  (:`Pressed`
    (bind _caninteract (`self.CanInteract`))
    (if _caninteract
      (set `self.InProgress` true)
      (`self.SetActorTickEnabled` true)
      (bind _asbp_side_scroller_character (cast `/Game/Blueprints/Characters/BP_SideScrollerCharacter` (`GameplayStatics.GetPlayerCharacter` 0)))
      (bind _output_get (set `self.Character` _asbp_side_scroller_character))
      (`/Game/Blueprints/Characters/BP_SideScrollerCharacter.Set Levitating` _output_get true)
      (`self.K2_SetActorRotation` (`self.Character`) (`self.GetClimbRotation`) false)
      (`self.K2_SetActorLocation` (`self.Character`) (`self.GetAbsoluteStart`) false false))))

(event `self.ReceiveTick`
  (params (DeltaSeconds :type "Float (single-precision)"))
  (if (`self.InProgress`)
    (`self.K2_AddActorWorldOffset` (`self.Character`) (* (`KismetMathLibrary.Normal` (- (`self.ClimbEnd`) (`self.ClimbStart`))) (* DeltaSeconds (`self.Speed`))) false false)
    (if (`self.GotToEnd`)
      (`self.K2_SetActorLocationAndRotation` (`self.Character`) (`self.GetAbsoluteDestination`) (`self.GetDestinationRotation`) false true)
      (`self.SetActorTickEnabled` false)
      (`self.SetActive` (`self.IsReusable`))
      (`/Game/Blueprints/Characters/BP_SideScrollerCharacter.Set Levitating` (`self.Character`) false)
      (set `self.InProgress` false))))

(fn `CanInteract`
  (returns (CanInteract :type Boolean))
  (bind _caninteract (`parent.CanInteract`))
  (return (and _caninteract (`self.IsActive`) (not (`self.InProgress`)))))

(fn `GetAbsoluteDestination`
  (returns (Destination :type "Vector Structure"))
  (return (+ (`self.K2_GetActorLocation`) (`self.Destination`))))

(fn `GetAbsoluteEnd`
  (returns (End :type "Vector Structure"))
  (return (+ (`self.K2_GetActorLocation`) (`self.ClimbEnd`))))

(fn `GetAbsoluteStart`
  (returns (Start :type "Vector Structure"))
  (return (+ (`self.K2_GetActorLocation`) (`self.ClimbStart`))))

(fn `GetClimbRotation`
  (returns (ReturnValue :type "Rotator Structure"))
  (return (`KismetMathLibrary.MakeRotationFromAxes` (`KismetMathLibrary.Cross_VectorVector` (- (`self.ClimbEnd`) (`self.ClimbStart`)) (* (`SceneComponent.GetForwardVector` (`self.Right`)) -1.0)))))

(fn `GetDestinationRotation`
  (returns (Rotation :type "Rotator Structure"))
  (return (`KismetMathLibrary.MakeRotationFromAxes` (`SceneComponent.GetForwardVector` (`self.DestinationForward`)))))

(fn `GotToEnd`
  (returns (ReturnValue :type Boolean))
  (return (< (`KismetMathLibrary.Dot_VectorVector` (`KismetMathLibrary.GetDirectionUnitVector` (`self.GetAbsoluteEnd`) (`self.GetAbsoluteStart`)) (`KismetMathLibrary.GetDirectionUnitVector` (`self.GetAbsoluteEnd`) (`self.K2_GetActorLocation` (`self.Character`)))) 0.0)))

(fn `SetActive`
  (params (IsActive :type Boolean))
  (bind _output_get (set `self.IsActive` IsActive))
  (if _output_get
    (`PrimitiveComponent.SetCollisionEnabled` (`self.InteractionTrigger`) "QueryAndPhysics")
    (else
      (`PrimitiveComponent.SetCollisionEnabled` (`self.InteractionTrigger`) "NoCollision"))))

(fn `UserConstructionScript`)