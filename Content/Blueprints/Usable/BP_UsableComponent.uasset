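; Usable component that runs the use lifecycle of its owning actor: start, interrupt and complete, each firing a call for that stage.
; Macros gate each step on active, in-progress and use-once state, with ExecutionType deciding whether a running use can be interrupted.
; Instant uses complete immediately and call complete-use twice, while both task types wait for TryComplete.
; Color-coded screen prints report attempts, naming instigator and owner.
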(fn `GetOwnerActorName`
  (returns (Name :type String))
  (return (`KismetSystemLibrary.GetObjectName` (`self.GetOwner`))))

(fn `Log`
  (params (Instigator :type "Pawn Object Reference") (Message :type String) (Error :type Boolean :default false))
  (`KismetSystemLibrary.PrintString` (`KismetStringLibrary.Concat_StrStr` "[" (`KismetSystemLibrary.GetObjectName` Instigator) "]" Message "[" (`self.GetOwnerActorName`) "]") true true (select `bool` Error :`false` (struct :`R` 0.173346 :`G` 1.0 :`B` 0.156186 :`A` 1.0) :`true` (struct :`R` 0.848958 :`B` 0.033207 :`A` 1.0) :!type "LinearColor Structure")))

(fn `TryComplete`
  (params (Instigator :type "Pawn Object Reference"))
  (`self.CanComplete`
    (:`Can Complete`
      (set `self.Completed` true)
      (set `self.CompletedOnce` true)
      (set `self.InProgress` false)
      (`self.OnCompleteUse` Instigator)
      (`self.Log` Instigator " successfuly completes use of "))
    (:`Cannot Complete`
      (`self.Log` Instigator " fails to complete use of " true))))

(fn `TryInterrupt`
  (params (Instigator :type "Pawn Object Reference"))
  (`self.CanInterrupt`
    (:`Can Interrupt`
      (set `self.InProgress` false)
      (`self.OnInterruptUse` Instigator)
      (`self.Log` Instigator " successfully interrupt use of "))
    (:`Cannot Interrupt`
      (`self.Log` Instigator " fails to interrupt use of " true))))

(fn `TryUse`
  (params (Instigator :type "Pawn Object Reference"))
  (`self.CanUse`
    (:`Can Use`
      (set `self.InProgress` true)
      (switch `/Game/Blueprints/Usable/EN_UsableExecution` (`self.ExecutionType`)
        (:`NewEnumerator0`
          (`self.OnStartUse` Instigator)
          (`self.TryComplete` Instigator)
          (`self.OnCompleteUse` Instigator))
        (:`NewEnumerator1`
          (`self.OnStartUse` Instigator :!label _label)
          (`self.Log` Instigator " starts using "))
        (:`NewEnumerator2`
          (goto _label))))
    (:`Cannot Use`
      (`self.Log` Instigator " fails to use " true))))