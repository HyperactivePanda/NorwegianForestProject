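; Base actor for usable world interactions, letting a character start or interrupt a use through a Usable component.
; Tagged trigger boxes register it with the overlapping BPI_Interactor and show the nearest key-bound hint text.
; Usable callbacks play or stop the Elin montage, optionally snap the instigator to tagged arrow points, and toggle hints.
; CheckCanInteract and empty OnPost events serve as extension points for children.
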(event `OnTriggerBeginOverlap`
  (params (OverlappedComponent :type "PrimitiveComponent Object Reference") (OtherActor :type "Actor Object Reference") (OtherComp :type "PrimitiveComponent Object Reference") (OtherBodyIndex :type Integer) (bFromSweep :type Boolean) (SweepResult :type "HitResult Structure (by ref)"))
  ;[1 1 1] Setup
  (bind _asbpi_interactor (cast `/Game/Blueprints/Usable/Interactions/BPI_Interactor` OtherActor))
  (`/Game/Blueprints/Usable/Interactions/BPI_Interactor.SetCurrentInteractable` _asbpi_interactor self)
  (bind _asbox_collision (cast `BoxComponent` OverlappedComponent))
  (set `self.CurrentTrigger` _asbox_collision)
  (bind _ascharacter (cast `Character` OtherActor))
  (`self.ShowHint` _ascharacter))

(event `OnTriggerEndOverlap`
  (params (OverlappedComponent :type "PrimitiveComponent Object Reference") (OtherActor :type "Actor Object Reference") (OtherComp :type "PrimitiveComponent Object Reference") (OtherBodyIndex :type Integer))
  ;[1 1 1] Setup
  (bind _asbpi_interactor (cast `/Game/Blueprints/Usable/Interactions/BPI_Interactor` OtherActor))
  (`/Game/Blueprints/Usable/Interactions/BPI_Interactor.SetCurrentInteractable` _asbpi_interactor null)
  (`self.HideHints`))

(event `self.ReceiveBeginPlay`
  ;[1 1 1] Setup
  (for _array_element (`self.FindAllTriggers`)
    (`|ExecutionSequence`
      (:`then_0`
        (add `PrimitiveComponent.OnComponentBeginOverlap` _array_element (delegate `OnTriggerBeginOverlap`)))
      (:`then_1`
        (add `PrimitiveComponent.OnComponentEndOverlap` _array_element (delegate `OnTriggerEndOverlap`))))
    (`self.HideHints`)))

(event `self.TryInteract`
  (params (Instigator :type "Character Object Reference"))
  ;[1 1 1] On atempting to interact
  (if (`/Game/Blueprints/Usable/BP_UsableComponent.InProgress` (`self.Usable`))
    (`/Game/Blueprints/Usable/BP_UsableComponent.TryInterrupt` (`self.Usable`) Instigator)
    (else
      (bind _caninteract (`self.CheckCanInteract` Instigator))
      (if _caninteract
        (`/Game/Blueprints/Usable/BP_UsableComponent.TryUse` (`self.Usable`) Instigator)))))

(event `self.Usable.OnStartUse`
  (params (Instigator :type "Character Object Reference"))
  ;[1 1 1] Usable callbacks
  (`self.StartMontage` Instigator)
  (`self.TrySnapInstigator` Instigator true)
  (`self.HideHints`)
  (`self.OnPostStartUse` Instigator))

(event `self.Usable.OnInterruptUse`
  (params (Instigator :type "Character Object Reference"))
  ;[1 1 1] Usable callbacks
  (`self.StopMontage` Instigator)
  (`self.TrySnapInstigator` Instigator)
  (`self.ShowHint` Instigator)
  (`self.OnPostInterruptUse` Instigator))

(event `self.Usable.OnCompleteUse`
  (params (Instigator :type "Character Object Reference"))
  ;[1 1 1] Usable callbacks
  (`self.StopMontage` Instigator)
  (`self.TrySnapInstigator` Instigator)
  (`self.ShowHint` Instigator)
  (`self.OnPostCompleteUse` Instigator))

(event `OnPostStartUse`
  (params (Instigator :type "Character Object Reference"))
  ;[1 1 1] Post usable callbacks
)

(event `OnPostInterruptUse`
  (params (Instigator :type "Character Object Reference"))
  ;[1 1 1] Post usable callbacks
)

(event `OnPostCompleteUse`
  (params (Instigator :type "Character Object Reference"))
  ;[1 1 1] Post usable callbacks
)

(fn `CheckCanInteract`
  (params (Instigator :type "Character Object Reference"))
  (returns (CanInteract :type Boolean))
  (return true))

(fn `ChooseHintText`
  (params (Instigator :type "Character Object Reference"))
  (returns (HintText :type "TextRenderComponent Object Reference"))
  (locals (ClosestHintText :type "TextRenderComponent Object Reference"))
  (bind _returnvalue (`self.K2_GetActorLocation` Instigator))
  (if (> (`KismetArrayLibrary.Array_Length` (`self.HintTexts`)) 0)
    (set `local.ClosestHintText` (`|GetArrayItem` (`self.HintTexts`)))
    (for _array_element (`self.HintTexts`)
      (if (< (`KismetMathLibrary.VSizeSquared` (- (`SceneComponent.K2_GetComponentLocation` _array_element) _returnvalue)) (`KismetMathLibrary.VSizeSquared` (- _returnvalue (`SceneComponent.K2_GetComponentLocation` (`local.ClosestHintText`)))))
        (set `local.ClosestHintText` _array_element)))
    (return (`local.ClosestHintText`))))

(fn `ChooseSnapPoint`
  (params (Instigator :type "Actor Object Reference") (OnUse :type Boolean))
  (returns (SnapPoint :type "ArrowComponent Object Reference"))
  (bind _returnvalue (select `bool` OnUse :`false` (`self.OnEndUseSnapPoints`) :`true` (`self.OnUseSnapPoints`)))
  (if (!= (`KismetArrayLibrary.Array_Length` _returnvalue) 0)
    (if (> (`KismetArrayLibrary.Array_Length` _returnvalue) 0)
      (return (`|GetArrayItem` _returnvalue)))))

(fn `CollectSnapPoints`
  (`|ExecutionSequence`
    (:`then_0`
      (for _array_element (`self.GetComponentsByTag` "/Script/Engine.ArrowComponent" "OnUse_SnapPoint")
        (bind _asarrow_component (cast `ArrowComponent` _array_element))
        (`KismetArrayLibrary.Array_Add` (`self.OnUseSnapPoints`) _asarrow_component)))
    (:`then_1`
      (for _array_element_2 (`self.GetComponentsByTag` "/Script/Engine.ArrowComponent" "OnEndUse_SnapPoint")
        (bind _asarrow_component_2 (cast `ArrowComponent` _array_element_2))
        (`KismetArrayLibrary.Array_Add` (`self.OnEndUseSnapPoints`) _asarrow_component_2)))))

(fn `FindAllTriggers`
  (returns (NewParam :type "Array of BoxComponent Object Reference"))
  (return (`self.GetComponentsByTag` "/Script/Engine.BoxComponent" "InteractionTrigger")))

(fn `GetHintText`
  (returns (Result :type Text))
  (return (`|FormatText` "UI_Interaction" (`KismetInputLibrary.Key_GetDisplayName` (`.Key` (break `InputActionKeyMapping` (`|GetArrayItem` (`InputSettings.GetActionMappingByName` (`InputSettings.GetInputSettings`) "UseObject"))))))))

(fn `GetIsInProgress`
  (returns (InProgress :type Boolean))
  (return (`/Game/Blueprints/Usable/BP_UsableComponent.InProgress` (`self.Usable`))))

(fn `HideHints`
  (for _array_element (`self.HintTexts`)
    (`SceneComponent.SetVisibility` _array_element false false)))

(fn `SetHintTexts`
  (bind _output_get (set `self.HintTexts` (`self.GetComponentsByTag` "/Script/Engine.TextRenderComponent" "HintText")))
  (for _array_element _output_get
    (`TextRenderComponent.K2_SetText` _array_element (`self.GetHintText`))))

(fn `ShowHint`
  (params (Instigator :type "Character Object Reference"))
  (bind _inprogress (`self.GetIsInProgress`))
  (if (not _inprogress)
    (`/Engine/EditorBlueprintResources/StandardMacros.IsValid` (`self.CurrentTrigger`)
      (:`Is Valid`
        (bind _hinttext (`self.ChooseHintText` Instigator))
        (`SceneComponent.SetVisibility` _hinttext true false)))))

(fn `StartMontage`
  (params (Instigator :type "Actor Object Reference"))
  (`/Engine/EditorBlueprintResources/StandardMacros.IsValid` (`self.Montage`)
    (:`Is Valid`
      (bind _asanim_bp_elin (cast `/Game/Characters/Elin/Animations/AnimBP_Elin` (`SkeletalMeshComponent.GetAnimInstance` (`self.GetComponentByClass` Instigator "/Script/Engine.SkeletalMeshComponent"))))
      (`/Game/Characters/Elin/Animations/AnimBP_Elin.PlayInteractionMontage` _asanim_bp_elin (`self.Montage`)))))

(fn `StopMontage`
  (params (Instigator :type "Actor Object Reference"))
  (`/Engine/EditorBlueprintResources/StandardMacros.IsValid` (`self.Montage`)
    (:`Is Valid`
      (bind _asanim_bp_elin (cast `/Game/Characters/Elin/Animations/AnimBP_Elin` (`SkeletalMeshComponent.GetAnimInstance` (`self.GetComponentByClass` Instigator "/Script/Engine.SkeletalMeshComponent"))))
      (`/Game/Characters/Elin/Animations/AnimBP_Elin.StopInteractionMontage` _asanim_bp_elin (`self.Montage`)))))

(fn `TrySnapInstigator`
  (params (Instigator :type "Actor Object Reference") (OnUse :type Boolean))
  (bind (_returnvalue_roll _returnvalue_pitch) (`KismetMathLibrary.BreakRotator` (`self.K2_GetActorRotation` Instigator)))
  (if (`self.ShouldSnapInstigator`)
    (bind _snappoint (`self.ChooseSnapPoint` Instigator OnUse))
    (`/Engine/EditorBlueprintResources/StandardMacros.IsValid` _snappoint
      (:`Is Valid`
        (bind _returnvalue (`SceneComponent.K2_GetComponentRotation` _snappoint))
        (`self.K2_SetActorLocationAndRotation` Instigator (`SceneComponent.K2_GetComponentLocation` _snappoint) (select `bool` (`self.OnlyZSnapRotation`) :`false` _returnvalue :`true` (`KismetMathLibrary.MakeRotator` _returnvalue_roll _returnvalue_pitch (.yaw _returnvalue))) false true)))))

(fn `UserConstructionScript`
  (`self.CollectSnapPoints`)
  (`self.SetHintTexts`))