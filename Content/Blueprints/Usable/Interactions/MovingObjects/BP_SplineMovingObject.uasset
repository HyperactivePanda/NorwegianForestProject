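; Usable object that a character pushes or pulls along a spline, with start and end callbacks when progress reaches either limit.
; While in use, it slows the instigator, locks movement-based rotation and disables mesh collision.
; Each tick, instigator speed and world-Y velocity sign advance normalized progress, which places the pivot and trigger on the spline.
; The instigator is then re-pinned at its saved mesh offset, with height taken from the spline.
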(event `self.OnPostStartUse`
  (params (Instigator :type "Character Object Reference"))
  (`parent.OnPostStartUse` Instigator)
  (bind _output_get (set `self.CurrentInstigator` Instigator))
  (`self.SaveInstigatorInitialSpeed` _output_get)
  (`self.SetCanInstigatorRotate` _output_get)
  (`self.SetInstigatorSpeed` _output_get true)
  (`self.CalcDistanceToInstigator` _output_get)
  (`self.SetCollision` false)
  (`self.SetActorTickEnabled` true))

(event `self.OnPostInterruptUse`
  (params (Instigator :type "Character Object Reference"))
  (`parent.OnPostInterruptUse` Instigator)
  (`self.SetCanInstigatorRotate` Instigator true)
  (`self.SetInstigatorSpeed` Instigator)
  (`self.SetCollision` true :!label _label)
  (`self.SetActorTickEnabled` false))

(event `self.OnPostCompleteUse`
  (params (Instigator :type "Character Object Reference"))
  (`parent.OnPostCompleteUse` Instigator)
  (`self.SetCanInstigatorRotate` Instigator true)
  (`self.SetInstigatorSpeed` Instigator)
  (goto _label))

(event `self.ReceiveTick`
  (params (DeltaSeconds :type "Float (single-precision)"))
  (`self.UpdateProgress` DeltaSeconds)
  (`self.SetPivotLocationAndRotation`)
  (`self.SetInstigatorLocation`)
  (`self.SetInstigatorRotation`))

(fn `CalcDistanceToInstigator`
  (params (Instigator :type "Character Object Reference"))
  (set `self.DeltaToInstigator` (- (`self.K2_GetActorLocation` Instigator) (`SceneComponent.K2_GetComponentLocation` (`self.MovingObjectMesh`)))))

(fn `ChooseSnapPoint`
  (params (Instigator :type "Actor Object Reference") (OnUse :type Boolean))
  (returns (SnapPoint :type "ArrowComponent Object Reference"))
  (locals (ClosedSnapPoint :type "ArrowComponent Object Reference"))
  (bind _returnvalue (`self.K2_GetActorLocation` Instigator))
  (if OnUse
    (set `local.ClosedSnapPoint` (`|GetArrayItem` (`self.OnUseSnapPoints`)))
    (for _array_element (`self.OnUseSnapPoints`)
      (if (< (`KismetMathLibrary.VSizeSquared` (- (`SceneComponent.K2_GetComponentLocation` _array_element) _returnvalue)) (`KismetMathLibrary.VSizeSquared` (- _returnvalue (`SceneComponent.K2_GetComponentLocation` (`local.ClosedSnapPoint`)))))
        (set `local.ClosedSnapPoint` _array_element)))
    (return (`local.ClosedSnapPoint`))))

(fn `GetHalfInstigatorHeight`
  (params (Instigator :type "Character Object Reference"))
  (returns (HalfHeight :type "Float (double-precision)"))
  (return (`CapsuleComponent.CapsuleHalfHeight` (`Character.CapsuleComponent` Instigator))))

(fn `SaveInstigatorInitialSpeed`
  (params (Instigator :type "Character Object Reference"))
  (set `self.InstigatorInitialSpeed` (`CharacterMovementComponent.MaxWalkSpeed` (`Character.CharacterMovement` Instigator))))

(fn `SetCanInstigatorRotate`
  (params (Instigator :type "Character Object Reference") (CanRotate :type Boolean))
  (set `CharacterMovementComponent.bOrientRotationToMovement` CanRotate (`Character.CharacterMovement` Instigator)))

(fn `SetCollision`
  (params (Collide :type Boolean))
  (`PrimitiveComponent.SetCollisionEnabled` (`self.MovingObjectMesh`) (select `bool` Collide :`false` "NoCollision" :`true` "QueryAndPhysics" :!type "ECollisionEnabled Enum")))

(fn `SetInstigatorLocation`
  (bind (_returnvalue_x _returnvalue_y _returnvalue_z) (`KismetMathLibrary.BreakVector` (`SplineComponent.FindLocationClosestToWorldLocation` (`self.Spline`) (`self.K2_GetActorLocation` (`self.CurrentInstigator`)) "World")))
  (bind (_returnvalue_x_2 _returnvalue_y_2) (`KismetMathLibrary.BreakVector` (+ (`SceneComponent.K2_GetComponentLocation` (`self.MovingObjectMesh`)) (`KismetMathLibrary.GreaterGreater_VectorRotator` (`self.DeltaToInstigator`) (`KismetMathLibrary.MakeRotFromX` (`SceneComponent.GetRightVector` (`self.MovingObjectMesh`)))))))
  (`self.K2_SetActorLocation` (`self.CurrentInstigator`) (`KismetMathLibrary.MakeVector` _returnvalue_x_2 _returnvalue_y_2 (+ _returnvalue_z (`self.GetHalfInstigatorHeight` (`self.CurrentInstigator`)))) false false))

(fn `SetInstigatorNotFall`
  (params (Instigator :type "Character Object Reference") (CanFall :type Boolean)))

(fn `SetInstigatorRotation`
  (bind (_deltatoinstigator_x _deltatoinstigator_y) (`KismetMathLibrary.BreakVector` (`self.DeltaToInstigator`)))
  (bind (_returnvalue_roll _returnvalue_pitch _returnvalue_yaw) (`KismetMathLibrary.BreakRotator` (`SceneComponent.K2_GetComponentRotation` (`self.MovingObjectMesh`))))
  (bind (_returnvalue_roll_2 _returnvalue_pitch_2) (`KismetMathLibrary.BreakRotator` (`self.K2_GetActorRotation` (`self.CurrentInstigator`))))
  (`self.K2_SetActorRotation` (`self.CurrentInstigator`) (`KismetMathLibrary.MakeRotator` _returnvalue_roll_2 _returnvalue_pitch_2 (* _returnvalue_yaw (`KismetMathLibrary.SignOfFloat` _deltatoinstigator_y))) false))

(fn `SetInstigatorSpeed`
  (params (Instigator :type "Character Object Reference") (Slow :type Boolean))
  (set `CharacterMovementComponent.MaxWalkSpeed` (select `bool` Slow :`false` (`self.InstigatorInitialSpeed`) :`true` (`self.InstigatorPullSpeed`)) (`Character.CharacterMovement` Instigator)))

(fn `SetPivotLocationAndRotation`
  (bind _returnvalue (`KismetMathLibrary.Lerp` 0.0 (`SplineComponent.GetSplineLength` (`self.Spline`)) (`self.CurrentProgress`)))
  (bind _returnvalue_2 (`SplineComponent.GetRotationAtDistanceAlongSpline` (`self.Spline`) _returnvalue "Local"))
  (bind _returnvalue_3 (`SplineComponent.GetLocationAtDistanceAlongSpline` (`self.Spline`) _returnvalue "Local"))
  (`SceneComponent.K2_SetRelativeLocationAndRotation` (`self.MovingPivot`) _returnvalue_3 _returnvalue_2 false false)
  (`SceneComponent.K2_SetRelativeLocationAndRotation` (`self.Trigger_01`) (+ _returnvalue_3 (`KismetMathLibrary.GreaterGreater_VectorRotator` (`self.TriggerLocationAlongSplineOffset`) (`KismetMathLibrary.MakeRotFromZ` (`SplineComponent.GetUpVectorAtDistanceAlongSpline` (`self.Spline`) _returnvalue "Local")))) _returnvalue_2 false false))

(fn `UpdateProgress`
  (params (DeltaTime :type "Float (double-precision)"))
  (bind _returnvalue (`CharacterMovementComponent.GetLastUpdateVelocity` (`Character.CharacterMovement` (`self.CurrentInstigator`))))
  (bind _output_get (set `self.CurrentProgress` (`KismetMathLibrary.FClamp` (+ (* (/ (`KismetMathLibrary.VSize` (* _returnvalue DeltaTime)) (`SplineComponent.GetSplineLength` (`self.Spline`))) (`KismetMathLibrary.SignOfFloat` (.y _returnvalue)) -1.0) (`self.CurrentProgress`)))))
  (if (== _output_get 0.0)
    (`self.OnGetToStart`)
    (elif (== _output_get 1.0)
      (`self.OnGetToEnd`))))

(fn `UserConstructionScript`
  (`parent.UserConstructionScript`)
  (`self.SetPivotLocationAndRotation`))