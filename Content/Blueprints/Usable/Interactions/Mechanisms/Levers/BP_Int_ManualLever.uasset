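; BP_Int_ManualLever is an interactable lever mechanism that the player moves by hand through axis input while using it.
; Starting use stores the instigator and enables input from player controller 0, while interrupting or completing use disables it.
; The RotateLever axis, scaled by PullSpeed and inverted, feeds MoveLever on every input update.
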(event `/Game/Blueprints/Usable/Interactions/BP_BaseInteraction.OnPostStartUse`
  (params (Instigator :type "Character Object Reference"))
  (`parent.OnPostStartUse` Instigator)
  (set `self.PawnInstigator` Instigator)
  (`self.EnableInput` (`GameplayStatics.GetPlayerController` 0)))

(event `/Game/Blueprints/Usable/Interactions/BP_BaseInteraction.OnPostInterruptUse`
  (params (Instigator :type "Character Object Reference"))
  (`parent.OnPostInterruptUse` Instigator)
  (`self.DisableInput` (`GameplayStatics.GetPlayerController` 0) :!label _label))

(event `/Game/Blueprints/Usable/Interactions/BP_BaseInteraction.OnPostCompleteUse`
  (params (Instigator :type "Character Object Reference"))
  (`parent.OnPostCompleteUse` Instigator)
  (goto _label))

(event `InputAxis|RotateLever`
  (params (AxisValue :type "Float (single-precision)"))
  (`self.MoveLever` (* AxisValue (`self.PullSpeed`) -1.0)))

(fn `UserConstructionScript`
  (`parent.UserConstructionScript`))