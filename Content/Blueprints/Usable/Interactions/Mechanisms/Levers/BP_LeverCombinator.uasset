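; BP_LeverCombinator is a lever mechanism that mixes the progress of several levers into summed values for shared outputs.
; A Levers map gives each lever an amplifier and a list of outputs.
; Each output's value is the sum of amplifier times progress across its linked levers, broadcast through OnOutputUpdate.
; It broadcasts all unique outputs on BeginPlay, then recomputes only a moved lever's outputs.
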(event `self.ReceiveBeginPlay`
  (bind _keys (`BlueprintMapLibrary.Map_Keys` (`self.Levers`)))
  (for _array_element _keys
    (`/Engine/EditorBlueprintResources/StandardMacros.IsValid` _array_element
      (:`Is Valid`
        (add `/Game/Blueprints/Usable/Interactions/Mechanisms/Levers/BP_Int_BaseLever.OnLeverMoved` _array_element (delegate `OnLeverMoved`)))))
  (`self.UpdateAllOutputs`))

(event `OnLeverMoved`
  (params (Interactable :type "/Game/Blueprints/Usable/Interactions/Mechanisms/Levers/BP_Int_BaseLever Object Reference") (Progress :type "Float (double-precision)"))
  (bind (_value _returnvalue) (`BlueprintMapLibrary.Map_Find` (`self.Levers`) Interactable))
  (if _returnvalue
    (`self.UpdateOutputs` (`.Outputs_14_7C4BE65B41FF0CCC0334CDA567FB0279` (break `/Game/Blueprints/Usable/Interactions/Mechanisms/Levers/ST_LeverCombinationPart` _value)))))

(fn `GetSumForOutput`
  (params (Output :type Integer))
  (returns (Sum :type "Float (double-precision)"))
  (locals (Result :type "Float (double-precision)"))
  (bind _keys (`BlueprintMapLibrary.Map_Keys` (`self.Levers`)))
  (for _array_element _keys
    (bind (_amplifier _outputs) (break `/Game/Blueprints/Usable/Interactions/Mechanisms/Levers/ST_LeverCombinationPart` (`BlueprintMapLibrary.Map_Find` (`self.Levers`) _array_element)))
    (if (`KismetArrayLibrary.Array_Contains` _outputs Output)
      (set `local.Result` (+ (* _amplifier (`/Game/Blueprints/Usable/Interactions/Mechanisms/Levers/BP_Int_BaseLever.GetCurrentProgress` _array_element)) (`local.Result`)))))
  (return (`local.Result`)))

(fn `UpdateAllOutputs`
  (locals (UniqueOutputs :type "Array of Integer"))
  (bind _values (`BlueprintMapLibrary.Map_Values` (`self.Levers`)))
  (for _array_element _values
    (for _array_element_2 (`.Outputs_14_7C4BE65B41FF0CCC0334CDA567FB0279` (break `/Game/Blueprints/Usable/Interactions/Mechanisms/Levers/ST_LeverCombinationPart` _array_element))
      (`KismetArrayLibrary.Array_AddUnique` (`local.UniqueOutputs`) _array_element_2)))
  (`self.UpdateOutputs` (`local.UniqueOutputs`)))

(fn `UpdateOutputs`
  (params (Outputs :type "Array of Integer"))
  (for _array_element Outputs
    (bind _sum (`self.GetSumForOutput` _array_element))
    (`self.OnOutputUpdate` _array_element _sum)))

(fn `UserConstructionScript`)