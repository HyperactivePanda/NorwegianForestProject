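; Usable lever Blueprint that swings between a start and end angle while in use.
; Starting use enables Tick and picks the pull direction from the pivot's pitch relative to both limits, heading toward the farther one.
; Tick feeds speed-scaled steps to MoveLever and tries to complete the use when it returns true; completion or interruption disables Tick.
; Construction rounds StartAt to a whole number before running the parent script.
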(event `self.OnPostStartUse`
  (params (Instigator :type "Character Object Reference"))
  (`parent.OnPostStartUse` Instigator)
  (`self.SetActorTickEnabled` true)
  (set `self.CurrentInstigator` Instigator)
  (`self.SetPullDirection`))

(event `self.OnPostInterruptUse`
  (params (Instigator :type "Character Object Reference"))
  (`parent.OnPostInterruptUse` Instigator)
  (`self.SetActorTickEnabled` false :!label _label))

(event `self.OnPostCompleteUse`
  (params (Instigator :type "Character Object Reference"))
  (`parent.OnPostCompleteUse` Instigator)
  (goto _label))

(event `self.ReceiveTick`
  (params (DeltaSeconds :type "Float (single-precision)"))
  (bind _completed (`self.MoveLever` (* DeltaSeconds (`self.PullDirection`) (`self.PullSpeed`))))
  (if _completed
    (`/Game/Blueprints/Usable/BP_UsableComponent.TryComplete` (`self.Usable`) (`self.CurrentInstigator`))))

(fn `SetPullDirection`
  (bind (_relativerotation_roll _relativerotation_pitch) (`KismetMathLibrary.BreakRotator` (`SceneComponent.RelativeRotation` (`self.Pivot`))))
  (bind (_relativerotation_roll_2 _relativerotation_pitch_2) (`KismetMathLibrary.BreakRotator` (`SceneComponent.RelativeRotation` (`self.Pivot`))))
  (set `self.PullDirection` (`KismetMathLibrary.SignOfFloat` (+ (- (`self.StartAngle`) _relativerotation_pitch_2) (- (`self.EndAngle`) _relativerotation_pitch)))))

(fn `UserConstructionScript`
  (set `self.StartAt` (`KismetMathLibrary.Conv_IntToDouble` (`KismetMathLibrary.Round` (`self.StartAt`))))
  (`parent.UserConstructionScript`))