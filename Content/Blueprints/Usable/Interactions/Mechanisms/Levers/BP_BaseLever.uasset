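; Base usable lever mechanism that pitches a pivot between a start and end angle.
; Starting use disables the side-scroller character's movement, and interrupting or completing use restores it.
; The construction script sets the initial pitch from a StartAt blend of both angles.
; MoveLever adds a clamped pitch delta, fires moved and at-start or at-end events, and returns whether a limit is reached.
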(event `self.OnPostStartUse`
  (params (Instigator :type "Character Object Reference"))
  (`parent.OnPostStartUse` Instigator)
  (bind _asbp_side_scroller_character (cast `/Game/Blueprints/Characters/BP_SideScrollerCharacter` Instigator))
  (`/Game/Blueprints/Characters/BP_SideScrollerCharacter.SetCanMove` _asbp_side_scroller_character false))

(event `self.OnPostInterruptUse`
  (params (Instigator :type "Character Object Reference"))
  (`parent.OnPostInterruptUse` Instigator)
  (bind _asbp_side_scroller_character (cast `/Game/Blueprints/Characters/BP_SideScrollerCharacter` Instigator))
  (`/Game/Blueprints/Characters/BP_SideScrollerCharacter.SetCanMove` _asbp_side_scroller_character true))

(event `self.OnPostCompleteUse`
  (params (Instigator :type "Character Object Reference"))
  (`parent.OnPostCompleteUse` Instigator)
  (bind _asbp_side_scroller_character (cast `/Game/Blueprints/Characters/BP_SideScrollerCharacter` Instigator))
  (`/Game/Blueprints/Characters/BP_SideScrollerCharacter.SetCanMove` _asbp_side_scroller_character true))

(fn `MoveLever`
  (params (Amount :type "Float (double-precision)"))
  (returns (Completed :type Boolean))
  (bind (_relativerotation_roll _relativerotation_pitch) (`KismetMathLibrary.BreakRotator` (`SceneComponent.RelativeRotation` (`self.Pivot`))))
  (bind _returnvalue (`KismetMathLibrary.ClampAngle` (+ Amount _relativerotation_pitch) (`KismetMathLibrary.FMin` (`self.StartAngle`) (`self.EndAngle`)) (`KismetMathLibrary.FMax` (`self.StartAngle`) (`self.EndAngle`))))
  (`SceneComponent.K2_SetRelativeRotation` (`self.Pivot`) (`KismetMathLibrary.MakeRotator` 0.0 _returnvalue) false false)
  (`self.OnLeverMoved`)
  (if (`KismetMathLibrary.NearlyEqual_FloatFloat` _returnvalue (`self.StartAngle`))
    (`self.OnLeverAtStart`)
    (elif (`KismetMathLibrary.NearlyEqual_FloatFloat` _returnvalue (`self.EndAngle`))
      (`self.OnLeverAtEnd`)
      (else
        (return false))))
  (return true))

(fn `UserConstructionScript`
  (`parent.UserConstructionScript`)
  (`SceneComponent.K2_SetRelativeRotation` (`self.Pivot`) (`KismetMathLibrary.MakeRotator` 0.0 (`KismetMathLibrary.Lerp` (`self.StartAngle`) (`self.EndAngle`) (`self.StartAt`))) false false))