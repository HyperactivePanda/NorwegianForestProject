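; Usable interaction that carries the instigating character along a spline from one end to the other, with a configurable allowed direction.
; The spline end nearest the current trigger sets the travel direction and gates whether interaction is allowed.
; During use it disables character movement and teleports the instigator along the spline each tick, completing the use at the far end.
; Walking mode is restored on completion or interruption, and snap points are chosen by proximity to the instigator.
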(event `self.OnPostStartUse`
  (params (Instigator :type "Character Object Reference"))
  (bind _output_get (set `self.CurrentInstigator` Instigator))
  (`self.SetInstigatorMovement` _output_get)
  (`self.SetActorTickEnabled` true)
  (`self.InitMovement`))

(event `self.OnPostInterruptUse`
  (params (Instigator :type "Character Object Reference"))
  (`self.SetInstigatorMovement` Instigator true)
  (`self.SetActorTickEnabled` false :!label _label))

(event `self.OnPostCompleteUse`
  (params (Instigator :type "Character Object Reference"))
  (`self.SetInstigatorMovement` Instigator true)
  (goto _label))

(event `self.ReceiveTick`
  (params (DeltaSeconds :type "Float (single-precision)"))
  (bind _inprogress (`self.GetIsInProgress`))
  (if _inprogress
    (bind _completed (`self.UpdateLocation` DeltaSeconds))
    (if _completed
      (`/Game/Blueprints/Usable/BP_UsableComponent.TryComplete` (`self.Usable`) (`self.CurrentInstigator`)))))

(fn `CheckCanInteract`
  (params (Instigator :type "Character Object Reference"))
  (returns (CanInteract :type Boolean))
  (bind _canmove (`self.CheckCanMoveByDirection`))
  (return _canmove))

(fn `CheckCanMoveByDirection`
  (returns (CanMove :type Boolean))
  (bind _returnvalue (`self.IsCloseToStart`))
  (switch `/Game/Blueprints/Usable/Interactions/CharacterMovement/EN_SplineMovementDirection` (`self.MovementDirection`)
    (:`NewEnumerator0`
      (return _returnvalue))
    (:`NewEnumerator1`
      (return (not _returnvalue)))
    (:`NewEnumerator2`
      (return true))))

(fn `ChooseSnapPoint`
  (params (Instigator :type "Actor Object Reference") (OnUse :type Boolean))
  (returns (SnapPoint :type "ArrowComponent Object Reference"))
  (locals (ClosedSnapPoint :type "ArrowComponent Object Reference"))
  (bind _returnvalue (`self.K2_GetActorLocation` Instigator))
  (bind _returnvalue_2 (select `bool` OnUse :`false` (`self.OnEndUseSnapPoints`) :`true` (`self.OnUseSnapPoints`)))
  (set `local.ClosedSnapPoint` (`|GetArrayItem` _returnvalue_2))
  (for _array_element _returnvalue_2
    (if (< (`KismetMathLibrary.VSizeSquared` (- (`SceneComponent.K2_GetComponentLocation` _array_element) _returnvalue)) (`KismetMathLibrary.VSizeSquared` (- _returnvalue (`SceneComponent.K2_GetComponentLocation` (`local.ClosedSnapPoint`)))))
      (set `local.ClosedSnapPoint` _array_element)))
  (return (`local.ClosedSnapPoint`)))

(fn `InitMovement`
  (if (`self.IsCloseToStart`)
    (set `self.MovementDirectionValue` 1.0)
    (set `self.CurrentDistanceOnSpline` 0.0)
    (else
      (set `self.MovementDirectionValue` -1.0)
      (set `self.CurrentDistanceOnSpline` (`SplineComponent.GetSplineLength` (`self.Spline`))))))

(fn `IsCloseToStart`
  (returns (ReturnValue :type Boolean))
  (bind _spline (`self.Spline`))
  (bind _returnvalue (`SceneComponent.K2_GetComponentLocation` (`self.CurrentTrigger`)))
  (return (< (`KismetMathLibrary.VSizeSquared` (- (`SplineComponent.GetLocationAtDistanceAlongSpline` (`self.Spline`) 0.0 "World") _returnvalue)) (`KismetMathLibrary.VSizeSquared` (- _returnvalue (`SplineComponent.GetLocationAtDistanceAlongSpline` _spline (`SplineComponent.GetSplineLength` _spline) "World"))))))

(fn `SetInstigatorLocation`)

(fn `SetInstigatorMovement`
  (params (Instigator :type "Character Object Reference") (Move :type Boolean))
  (`CharacterMovementComponent.SetMovementMode` (`Character.CharacterMovement` Instigator) (select `bool` Move :`false` "MOVE_None" :`true` "MOVE_Walking" :!type "EMovementMode Enum") 0))

(fn `UpdateLocation`
  (params (DeltaSeconds :type "Float (double-precision)"))
  (returns (Completed :type Boolean))
  (bind _returnvalue (`SplineComponent.GetSplineLength` (`self.Spline`)))
  (bind _output_get (set `self.CurrentDistanceOnSpline` (`KismetMathLibrary.FClamp` (+ (* DeltaSeconds (`self.MovementSpeed`) (`self.MovementDirectionValue`)) (`self.CurrentDistanceOnSpline`)) 0.0 _returnvalue)))
  (`self.K2_SetActorLocation` (`self.CurrentInstigator`) (`SplineComponent.GetLocationAtDistanceAlongSpline` (`self.Spline`) (`self.CurrentDistanceOnSpline`) "World") false true)
  (if (and (`KismetMathLibrary.NearlyEqual_FloatFloat` _output_get) (== -1.0 (`self.MovementDirectionValue`)))
    (`self.OnGetToStart`)
    (elif (and (`KismetMathLibrary.NearlyEqual_FloatFloat` _output_get _returnvalue) (== 1.0 (`self.MovementDirectionValue`)))
      (`self.OnGetToEnd`)
      (else
        (return false))))
  (return true))

(fn `UserConstructionScript`
  (`parent.UserConstructionScript`))